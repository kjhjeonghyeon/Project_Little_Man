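; BP_OnOff2radio is a radio-style music zone that plays a song while a Player-tagged actor is inside its Trigger volume.
; Entering spawns the sound attached to the Trigger and fades it in, and leaving fades the stored audio component out.
; Shortly after BeginPlay it also checks existing overlaps, so music starts if the player begins inside.
; Each entry spawns a new audio component rather than reusing the previous one.
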(event `self.ReceiveBeginPlay`
  (`KismetSystemLibrary.Delay` 0.1)
  (for _array_element (`PrimitiveComponent.GetOverlappingActors` (`self.Trigger`) null)
    (if (`self.ActorHasTag` _array_element "Player")
      (bind _returnvalue (`GameplayStatics.SpawnSoundAttached` "/Game/User/dg/sounddg/ariatti_dibo_thankyou_3.ariatti_dibo_thankyou_3" (`self.Trigger`) "None" (0.0 0.0 0.0) (struct) "KeepRelativeOffset" false 1.0 1.0 0.0 "/Game/User/dg/sounddg/dobpthankyou.dobpthankyou" null))
      (bind _output_get (set `self.Music` _returnvalue))
      (`AudioComponent.FadeIn` _output_get 0.5 1.0 0.0 "Linear"))))

(event `self.Trigger.OnComponentBeginOverlap`
  (params (OverlappedComponent :type "PrimitiveComponent Object Reference") (OtherActor :type "Actor Object Reference") (OtherComp :type "PrimitiveComponent Object Reference") (OtherBodyIndex :type Integer) (bFromSweep :type Boolean) (SweepResult :type "HitResult Structure (by ref)"))
  (if (`self.ActorHasTag` OtherActor "Player")
    (bind _returnvalue (`GameplayStatics.SpawnSoundAttached` "/Game/User/dg/sounddg/ariatti_dibo_thankyou_3.ariatti_dibo_thankyou_3" (`self.Trigger`) "None" (0.0 0.0 0.0) (struct) "KeepRelativeOffset" false 1.0 1.0 0.0 "/Game/User/dg/sounddg/dobpthankyou.dobpthankyou" null))
    (bind _output_get (set `self.Music` _returnvalue))
    (`AudioComponent.FadeIn` _output_get 0.5 1.0 0.0 "Linear")))

(event `self.Trigger.OnComponentEndOverlap`
  (params (OverlappedComponent :type "PrimitiveComponent Object Reference") (OtherActor :type "Actor Object Reference") (OtherComp :type "PrimitiveComponent Object Reference") (OtherBodyIndex :type Integer))
  (if (`self.ActorHasTag` OtherActor "Player")
    (bind _music (`self.Music`)
      (:`then`
        (`AudioComponent.FadeOut` _music 0.5 0.0 "Linear"))
      (:`else`))))

(fn `UserConstructionScript`)