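; BP_Item is a pickup item actor for a pickup system, with its mesh set from ItemModelToPlace in the construction script.
; Pressing E gets overlapping BP_Item actors and sends PickupMessage to those implementing BPI_Items.
; A separate Pickup event prints a debug message, waits one tick and destroys the item.
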(event `/Game/User/My/Pickingup_system/BPI_Items.Pickup`
  (`KismetSystemLibrary.PrintString` "Item Picked")
  (`KismetSystemLibrary.DelayUntilNextTick`)
  (`self.K2_DestroyActor`))

(event `Key|E`
  (params (Key :type "Key Structure"))
  (:`Pressed`
    (for _array_element (`self.GetOverlappingActors` "BP_Item_C")
      (if (`KismetSystemLibrary.DoesImplementInterface` _array_element "/Game/User/My/Pickingup_system/BPI_Items.BPI_Items_C")
        (message `/Game/User/My/Pickingup_system/BPI_Items.Pickup` _array_element)))))

(fn `UserConstructionScript`
  (`StaticMeshComponent.SetStaticMesh` (`self.ItemModelToPlace`)))