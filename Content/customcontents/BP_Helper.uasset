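; BP_Helper is a set of vector and rotation helper functions.
; The move functions offset a vector along world Z for up and down, or along a rotation's forward or right vector for backward, left and right.
; MovevectorForward currently returns its input unchanged, as its forward offset is computed but left unconnected.
; Reversenormal builds a rotation from a normal's X axis and takes its delta against a fixed 180-degree rotator.
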(fn `Movevectorbackward`
  (params (invector :type "Vector Structure") (inrotation :type "Rotator Structure") (subtractvalue :type "Float (double-precision)"))
  (returns (returnvalue :type "Vector Structure"))
  (return (- invector (* (`KismetMathLibrary.GetForwardVector` inrotation) subtractvalue))))

(fn `MoveVectorDownward`
  (params (invector :type "Vector Structure") (subtractvalue :type "Float (double-precision)"))
  (returns (ReturnNode :type "Vector Structure"))
  (return (- invector (`KismetMathLibrary.MakeVector` 0.0 0.0 subtractvalue))))

(fn `MovevectorForward`
  (params (Invector :type "Vector Structure") (Inrotation :type "Rotator Structure") (Addvalue :type "Float (double-precision)"))
  (returns (Returnvlaue :type "Vector Structure"))
  (return (+ Invector (0.0 0.0 0.0))))

(fn `Movevectorleft`
  (params (invector :type "Vector Structure") (inrotation :type "Rotator Structure") (movevalue :type "Float (double-precision)"))
  (returns (returnvalue :type "Vector Structure"))
  (return (- invector (* (`KismetMathLibrary.GetRightVector` inrotation) movevalue))))

(fn `movevectorright`
  (params (invector :type "Vector Structure") (inrotation :type "Rotator Structure") (`move value` :type "Float (double-precision)"))
  (returns (Returnvalue :type "Vector Structure"))
  (return (+ invector (* (`KismetMathLibrary.GetRightVector` inrotation) `move value`))))

(fn `MovevectorUpword`
  (params (INvector :type "Vector Structure") (Addvalue :type "Float (double-precision)"))
  (returns (ReturnValue :type "Vector Structure"))
  (return (+ INvector (`KismetMathLibrary.MakeVector` 0.0 0.0 Addvalue))))

(fn `reversenormal`
  (params (innormal :type "Vector Structure"))
  (returns (returnvalue :type "Rotator Structure"))
  (return (`KismetMathLibrary.NormalizedDeltaRotator` (`KismetMathLibrary.MakeRotFromX` innormal) (struct :`Yaw` 180.0))))