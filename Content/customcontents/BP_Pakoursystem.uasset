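; Parkour component that probes for walls in front of its owning actor, with only the detection stage built so far.
; TriggerPakkour calls Detectwall, which stacks forward sphere traces upward from below the actor's location until one hits, returning location and reversed normal.
; Scanwall line-traces top-down along that normal, storing the first hit and wall rotation, but nothing calls it yet.
; All traces draw debug shapes.
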(fn `Detectwall`
  (returns (returnvalue :type Boolean) (`hit location` :type "Vector Structure") (reversenormal :type "Rotator Structure"))
  (bind _returnvalue (`self.GetOwner`))
  (for _index (range 8)
    (bind _returnvalue_2 (`/Game/customcontents/BP_Helper.MovevectorUpword` (`/Game/customcontents/BP_Helper.MoveVectorDownward` (`Actor.K2_GetActorLocation` _returnvalue) 60.0) (* _index 20.0)))
    (bind (_outhit _returnvalue_3) (`KismetSystemLibrary.SphereTraceSingle` :`Start` (`/Game/customcontents/BP_Helper.Movevectorbackward` _returnvalue_2 (`Actor.K2_GetActorRotation` _returnvalue) 30.0) :`End` (+ _returnvalue_2 (* (`Actor.GetActorForwardVector` _returnvalue) 200.0)) :`Radius` 10.0 :`TraceChannel` "TraceTypeQuery1" :`DrawDebugType` "ForOneFrame"))
    (if _returnvalue_3
      (`|ExecutionSequence`
        (:`then_0`
          (break))
        (:`then_1`
          (bind (_bblockinghit _binitialoverlap _time _distance _location _impactpoint _normal) (`GameplayStatics.BreakHitResult` _outhit))
          (return _bblockinghit _location (`/Game/customcontents/BP_Helper.reversenormal` _normal)))))))

(fn `scanwall`
  (params (detectlocation :type "Vector Structure") (reversenormal :type "Rotator Structure"))
  (locals (ScanHitResult :type "HitResult Structure"))
  (bind _reversenormal (`local.reversenormal`))
  (for _index (range 30)
    (bind _returnnode (`/Game/customcontents/BP_Helper.MoveVectorDownward` (`/Game/customcontents/BP_Helper.MovevectorUpword` (`local.detectlocation`) 300.0) (* _index 10)))
    (bind (_outhit _returnvalue) (`KismetSystemLibrary.LineTraceSingle` :`Start` (`/Game/customcontents/BP_Helper.Movevectorbackward` _returnnode _reversenormal 20.0) :`End` (`/Game/customcontents/BP_Helper.MovevectorForward` _returnnode _reversenormal 80.0) :`TraceChannel` "TraceTypeQuery1" :`DrawDebugType` "ForOneFrame"))
    (if _returnvalue
      (set `local.ScanHitResult` _outhit)
      (break)))
  (set `self.Wallrotation` (`/Game/customcontents/BP_Helper.reversenormal` (`.Normal` (`GameplayStatics.BreakHitResult` (`local.ScanHitResult`))))))

(fn `TriggerPakkour`
  (`self.Detectwall`))